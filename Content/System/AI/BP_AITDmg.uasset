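; AI controller for a damage-dealer TestAI pawn that fights a boss.
; On begin play it runs the BTTDmg behavior tree, then after a short delay sets the pawn's Boss as blackboard FollowTarget.
; AutoAttack range-checks the boss, subtracts random damage with a crit chance from its HP, adds aggro through the game state and returns whether in range.
; The aggro value rolls its crit separately, so it can differ from damage dealt.
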(event `self.ReceiveBeginPlay`
  (bind (_astest_ai _bsuccess) (cast `/Game/System/Actors/TestAI` (`self.K2_GetPawn` self) :!pure true))
  (`self.RunBehaviorTree` "/Game/System/AI/BTTDmg.BTTDmg")
  (if _bsuccess
    (set `self.ControlledActor_0` _astest_ai)
    (`KismetSystemLibrary.Delay` 1.3)
    (`BlackboardComponent.SetValueAsObject` (`AIBlueprintHelperLibrary.GetBlackboard` null) "FollowTarget" (`/Game/System/Actors/TestAI.Boss` (`self.ControlledActor_0`)))))

(fn `Auto Attack `
  (returns (InRange :type Boolean))
  (locals (random :type Integer :default 0))
  (bind _boss (`/Game/System/Actors/TestAI.Boss` (`self.ControlledActor_0`)))
  (bind _hp (`/Game/System/Actors/TestBoss.HP` _boss))
  (bind _returnvalue (<= (`self.GetDistanceTo` (`self.ControlledActor_0`) (`/Game/System/Actors/TestAI.Boss` (`self.ControlledActor_0`))) 400.0))
  (bind _returnvalue_2 (`KismetMathLibrary.SelectInt` (`KismetMathLibrary.FTrunc` (* (/ (`local.random`) 100.0) 250.0)) (`local.random`) (<= (`KismetMathLibrary.RandomIntegerInRange` 0 100) 15)))
  (if _returnvalue
    (set `local.random` (`KismetMathLibrary.RandomIntegerInRange` 10 30))
    (set `/Game/System/Actors/TestBoss.HP` (`KismetMathLibrary.Clamp` (- _hp _returnvalue_2) 0 _hp) _boss)
    (`/Game/System/Controllers/BP_GameState.AddValueToAggro` (`/Game/System/Actors/TestAI.As BP Game State` (`self.ControlledActor_0`)) (`self.ControlledActor_0`) _returnvalue_2)
    (return _returnvalue)
    (else
      (return _returnvalue))))

(fn `UserConstructionScript`)