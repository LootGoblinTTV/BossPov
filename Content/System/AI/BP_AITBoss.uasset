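; BP_AITBoss is the AI controller for the TestBoss pawn, running the BTTBoss behavior tree and caching the controlled boss on BeginPlay.
; Its AutoAttack event subtracts random damage directly from the HP of the boss's current target, clamped at zero.
; CastSpell maps a spell index to a boss ability, with only the first spell wired up.
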(event `self.ReceiveBeginPlay`
  (`self.RunBehaviorTree` "/Game/System/AI/BTTBoss.BTTBoss")
  (set `self.As Test Boss` (cast `/Game/System/Actors/TestBoss` (`self.K2_GetPawn` self) :!pure true)))

(event `AutoAttack`
  (bind _hp (`/Game/System/Actors/TestAI.HP` (`/Game/System/Actors/TestBoss.Target` (`self.As Test Boss`))))
  (set `/Game/System/Actors/TestAI.HP` (`KismetMathLibrary.Clamp` (- _hp (`KismetMathLibrary.RandomIntegerInRange` 10 30)) 0 _hp) (`/Game/System/Actors/TestBoss.Target` (`self.As Test Boss`))))

(fn `CastSpell`
  (params (Spell :type Integer))
  (switch `int` Spell
    (:`1`
      (`/Game/System/Actors/TestBoss.CastFirstSpell` (`self.As Test Boss`)))))

(fn `UserConstructionScript`)