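; AI controller for a healer TestAI pawn, running the BTTHealer behavior tree and caching all TestAI actors on BeginPlay.
; FindAndReturnTargetToHeal selects the living, injured actor with the lowest HP from that cached list.
; HealTarget restores random HP, capped at 100, to a target within range and adds aggro to the healer through the game state.
; The heal, debug print and aggro each roll their random amount separately.
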(event `self.ReceiveBeginPlay`
  (`self.RunBehaviorTree` "/Game/System/AI/BTTHealer.BTTHealer")
  (bind _astest_ai (cast `/Game/System/Actors/TestAI` (`self.K2_GetPawn` self)))
  (set `self.ControlledActor_0` _astest_ai)
  (bind _outactors (`GameplayStatics.GetAllActorsOfClass` "/Game/System/Actors/TestAI.TestAI_C"))
  (set `self.Players` _outactors))

(fn `FindAndReturnTargetToHeal`
  (returns (`Success?` :type Boolean) (TargetToHeal :type "/Game/System/Actors/TestAI Object Reference"))
  (set `self.Target ToHeal` null)
  (for _array_element (`self.Players`)
    (if (`KismetSystemLibrary.IsValid` _array_element)
      (if (!= (`/Game/System/Actors/TestAI.HP` _array_element) 0)
        (bind _target_toheal (`self.Target ToHeal`)
          (:`then`
            (bind _hp (`/Game/System/Actors/TestAI.HP` _array_element))
            (bind _returnvalue (< _hp 100))
            (if (and _returnvalue (< _hp (`/Game/System/Actors/TestAI.HP` _target_toheal)))
              (set `self.Target ToHeal` _array_element)))
          (:`else`
            (if _returnvalue
              (set `self.Target ToHeal` _array_element)))))))
  (bind _target_toheal_2 (`self.Target ToHeal`)
    (:`then`
      (return true _target_toheal_2))
    (:`else`
      (return false null))))

(fn `HealTarget`
  (returns (Success :type Boolean))
  (bind _returnvalue (`KismetMathLibrary.RandomIntegerInRange` 30 50))
  (bind _returnvalue_2 (+ (`/Game/System/Actors/TestAI.HP` (`self.Target ToHeal`)) _returnvalue))
  (if (<= (`self.GetDistanceTo` (`self.ControlledActor_0`) (`self.Target ToHeal`)) 800.0)
    (set `/Game/System/Actors/TestAI.HP` (`KismetMathLibrary.Clamp` _returnvalue_2 0 100) (`self.Target ToHeal`))
    (`KismetSystemLibrary.PrintString` (`KismetStringLibrary.Concat_StrStr` "Heal" (`KismetStringLibrary.Conv_IntToString` _returnvalue_2)))
    (`/Game/System/Controllers/BP_GameState.AddValueToAggro` (`/Game/System/Actors/TestAI.As BP Game State` (`self.ControlledActor_0`)) (`self.ControlledActor_0`) _returnvalue)
    (return true)
    (else
      (return false))))

(fn `UserConstructionScript`)