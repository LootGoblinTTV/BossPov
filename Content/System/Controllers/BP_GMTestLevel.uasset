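; BP_GMTestLevel is a test-level controller that periodically drops an area damage test actor on AI characters.
; BeginPlay caches every TestAI actor in the level.
; Tick uses latent Delays as a repeating timer, spawning AoeDmgTest at a random cached AI's location about every 15 seconds.
; Each spawned AoE is stored and destroyed 5 seconds later.
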(event `self.ReceiveBeginPlay`
  (bind _outactors (`GameplayStatics.GetAllActorsOfClass` "/Game/System/Actors/TestAI.TestAI_C"))
  (set `self.Testai` _outactors))

(event `self.ReceiveTick`
  (params (DeltaSeconds :type "Float (single-precision)"))
  (`KismetSystemLibrary.Delay` 15.0)
  (`self.SpawnTEST`)
  (`KismetSystemLibrary.Delay` 5.0)
  (`self.K2_DestroyActor` (`self.Aoe`)))

(fn `SpawnTEST`
  (bind _returnvalue_location (`KismetMathLibrary.BreakTransform` (`self.GetTransform` (`KismetArrayLibrary.Array_Random` (`self.Testai`)))))
  (bind _returnvalue (`|SpawnActorFromClass` "/Game/System/Actors/AoeDmgTest.AoeDmgTest_C" (`KismetMathLibrary.MakeTransform` _returnvalue_location) "Undefined" "MultiplyWithRoot" null null))
  (set `self.Aoe` _returnvalue))

(fn `UserConstructionScript`)