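; Game state that tracks each TestAI actor's aggro toward the TestBoss and steers the boss's target.
; A second after BeginPlay it caches the boss, seeds an actor-to-aggro map at zero and shows the aggro widget.
; AddValueToAggro accumulates threat per actor.
; AggroOrder ranks entries by repeatedly extracting the maximum from a copy, then retargets the boss when the leader differs from its current target.
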(event `self.ReceiveBeginPlay`
  (`KismetSystemLibrary.Delay` 1.0)
  (bind _returnvalue (`GameplayStatics.GetActorOfClass` "/Game/System/Actors/TestBoss.TestBoss_C"))
  (set `self.Boss` _returnvalue)
  (bind _outactors (`GameplayStatics.GetAllActorsOfClass` "/Game/System/Actors/TestAI.TestAI_C"))
  (for _array_element _outactors
    (`BlueprintMapLibrary.Map_Add` (`self.AIPlayersAggrometter`) _array_element))
  (bind _returnvalue_2 (`|CreateWidget` "/Game/UI/Agrometter/W_AggroHolder.W_AggroHolder_C" (`GameplayStatics.GetPlayerController` 0)))
  (`UserWidget.AddToViewport` _returnvalue_2 0))

(event `SetAggrometer`
  (bind _keys (`BlueprintMapLibrary.Map_Keys` (`self.AIPlayersAggrometter`)))
  (for _ _keys
    _))

(fn `AddValueToAggro`
  (params (Actor :type "/Game/System/Actors/TestAI Object Reference (by ref)") (Value :type "Integer (by ref)"))
  (bind (_value _returnvalue) (`BlueprintMapLibrary.Map_Find` (`self.AIPlayersAggrometter`) Actor))
  (if _returnvalue
    (`BlueprintMapLibrary.Map_Add` (`self.AIPlayersAggrometter`) (`local.Actor`) (+ (`local.Value`) _value))
    (`KismetSystemLibrary.LogString` (`KismetStringLibrary.Concat_StrStr` (`KismetSystemLibrary.GetDisplayName` (`local.Actor`)) (`KismetStringLibrary.Conv_IntToString` (`local.Value`))))
    (else
      (`BlueprintMapLibrary.Map_Add` (`self.AIPlayersAggrometter`) (`local.Actor`) (`local.Value`))
      (`KismetSystemLibrary.LogString` (`KismetStringLibrary.Concat_StrStr` "New" (`KismetSystemLibrary.GetDisplayName` (`local.Actor`)))))))

(fn `AggroOrder`
  (returns (AggroOrderIndex :type "Array of Integer"))
  (locals (calc :type "Array of Integer"))
  (bind _indexofmaxvalue (`KismetMathLibrary.MaxOfIntArray` (`local.calc`)))
  (`KismetArrayLibrary.Array_Clear` (`self.AggroOrderIndex`))
  (bind _values (`BlueprintMapLibrary.Map_Values` (`self.AIPlayersAggrometter`)))
  (set `local.calc` _values)
  (for _ (range 1 (+ (`BlueprintMapLibrary.Map_Length` (`self.AIPlayersAggrometter`)) 1))
    (`KismetArrayLibrary.Array_Add` (`self.AggroOrderIndex`) _indexofmaxvalue)
    (`KismetArrayLibrary.Array_Set` (`local.calc`) _indexofmaxvalue -1))
  (`self.CheckIfTargetChaged`)
  (bind _values_2 (`BlueprintMapLibrary.Map_Values` (`self.AIPlayersAggrometter`)))
  (set `self.MaxAggroValue` (`.MaxValue` (`KismetMathLibrary.MaxOfIntArray` _values_2)))
  (return (`self.AggroOrderIndex`)))

(fn `CheckIfTargetChaged`
  (bind _keys (`BlueprintMapLibrary.Map_Keys` (`self.AIPlayersAggrometter`)))
  (bind _output (`|GetArrayItem` _keys (`|GetArrayItem` (`self.AggroOrderIndex`))))
  (if (not (== (`/Game/System/Actors/TestBoss.Target` (`self.Boss`)) _output))
    (`/Game/System/Actors/TestBoss.SetNewTarget` (`self.Boss`) _output))
  (return))

(fn `GetHighestAggro`
  (returns (Output :type "/Game/System/Actors/TestAI Object Reference") (Calc1 :type Integer))
  (locals (Calc :type Integer) (index :type Integer))
  (bind _values (`BlueprintMapLibrary.Map_Values` (`self.AIPlayersAggrometter`)))
  (for (_array_element _array_index) _values
    (if (> _array_element (`local.Calc`))
      (set `local.Calc` _array_element)
      (set `local.index` _array_index)))
  (bind _keys (`BlueprintMapLibrary.Map_Keys` (`self.AIPlayersAggrometter`)))
  (return (`|GetArrayItem` _keys (`local.index`)) (`local.Calc`)))

(fn `UserConstructionScript`)